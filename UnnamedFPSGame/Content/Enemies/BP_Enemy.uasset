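; Enemy actor that attacks the first-person player character whenever PawnSensing sees it.
; On sight it sets its rotation from a look-at whose start and target are both the player's location.
; A CanAttack gate with a half-second delay limits attacks, each spawning a projectile and applying damage directly, independent of any hit.
; FollowPlayer holds AI move-to chase logic, but its only call here is unreachable.
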(event `self.PawnSensing.OnSeePawn`
  (params (Pawn :type "Pawn Object Reference"))
  (bind _asbp_first_person_character (cast `/Game/FirstPerson/Blueprints/BP_FirstPersonCharacter` Pawn))
  (`self.K2_SetActorRotation` (`KismetMathLibrary.FindRelativeLookAtRotation` (`KismetMathLibrary.Conv_VectorToTransform` (`self.K2_GetActorLocation` _asbp_first_person_character)) (`self.K2_GetActorLocation` _asbp_first_person_character)))
  (if (`self.canAttack`)
    (`|SpawnActorFromClass` "/Game/FirstPerson/Blueprints/BP_FirstPersonProjectile.BP_FirstPersonProjectile_C" (`SceneComponent.K2_GetComponentToWorld` (`self.SpawnProjectileLocation`)) "Undefined" "MultiplyWithRoot" null null)
    (`GameplayStatics.ApplyDamage` _asbp_first_person_character 1.0)
    (set `self.canAttack` false)
    (`KismetSystemLibrary.Delay` 0.5)
    (set `self.canAttack` true)))

(event `FollowPlayer`
  (if (`self.isSeeingPlayer`)
    (`|AIMoveTo` self (0.0 0.0 0.0) (`GameplayStatics.GetPlayerCharacter` 0))))

(fn `UserConstructionScript`)