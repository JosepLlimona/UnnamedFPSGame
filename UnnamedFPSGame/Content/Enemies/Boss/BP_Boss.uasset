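; BP_Boss is a boss enemy that shows its health through a WBP_EnemyHealth widget component.
; Any damage is multiplied before being subtracted from health, then the widget is updated.
; At zero health it destroys every BP_tentacle actor in the level along with itself.
; Pawn sensing snaps its rotation to face a seen first-person player character.
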(event `self.ReceiveBeginPlay`
  (bind _aswbp_enemy_health (cast `/Game/Enemies/WBP_EnemyHealth` (`WidgetComponent.GetUserWidgetObject` (`self.Widget`))))
  (bind _output_get (set `self.WBP Enemy Health` _aswbp_enemy_health))
  (set `/Game/Enemies/WBP_EnemyHealth.CurrentHealth` (`self.CurrentHealth`) _output_get)
  (set `/Game/Enemies/WBP_EnemyHealth.MaxHealth` (`self.MaxHealth`) _output_get))

(event `self.ReceiveAnyDamage`
  (params (Damage :type "Float (single-precision)") (DamageType :type "DamageType Object Reference") (InstigatedBy :type "Controller Object Reference") (DamageCauser :type "Actor Object Reference"))
  (bind _output_get (set `self.CurrentHealth` (- (`self.CurrentHealth`) (* Damage 5.0))))
  (`/Game/Enemies/WBP_EnemyHealth.UpdateHealth` (`self.WBP Enemy Health`) _output_get)
  (if (<= (`self.CurrentHealth`) 0)
    (bind _outactors (`GameplayStatics.GetAllActorsOfClass` "/Game/Enemies/Boss/BP_tentacle.BP_tentacle_C"))
    (for _array_element _outactors
      (`self.K2_DestroyActor` _array_element))
    (`self.K2_DestroyActor`)))

(event `self.PawnSensing.OnSeePawn`
  (params (Pawn :type "Pawn Object Reference"))
  (cast `/Game/FirstPerson/Blueprints/BP_FirstPersonCharacter` Pawn)
  (`self.K2_SetActorRotation` (`KismetMathLibrary.FindLookAtRotation` (`self.K2_GetActorLocation`) (`self.K2_GetActorLocation` Pawn))))

(fn `UserConstructionScript`)