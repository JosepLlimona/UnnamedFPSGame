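; BP_FIRE is an enemy character with a health bar widget shown only when the player is within range.
; Damage is multiplied before reducing health and updating the bar; death spawns random ammo or health pickup, then destroys the actor.
; Player capsule overlap plays a hit sound and calls ApplyDamage on itself with no amount set.
; Attack plays a cast montage with empty notify handling, alongside ideal-range and walk-speed helper functions.
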(event `self.ReceiveTick`
  (params (DeltaSeconds :type "Float (single-precision)"))
  (bind _asbp_first_person_character (cast `/Game/FirstPerson/Blueprints/BP_FirstPersonCharacter` (`GameplayStatics.GetPlayerCharacter` 0)))
  (if (<= (`KismetMathLibrary.Vector_Distance` (`self.K2_GetActorLocation`) (`self.K2_GetActorLocation` _asbp_first_person_character)) (`self.WidgetRange`))
    (`SceneComponent.SetVisibility` (`self.Widget`) true false)
    (else
      (`SceneComponent.SetVisibility` (`self.Widget`) false false))))

(event `self.ReceiveBeginPlay`
  (bind _aswbp_enemy_health (cast `/Game/Enemies/WBP_EnemyHealth` (`WidgetComponent.GetUserWidgetObject` (`self.Widget`))))
  (bind _output_get (set `self.WBP Enemy Health` _aswbp_enemy_health))
  (set `/Game/Enemies/WBP_EnemyHealth.CurrentHealth` (`self.CurrentHealth`) _output_get)
  (set `/Game/Enemies/WBP_EnemyHealth.MaxHealth` (`self.MaxHealth`) _output_get))

(event `self.Capsule.OnComponentBeginOverlap`
  (params (OverlappedComponent :type "PrimitiveComponent Object Reference") (OtherActor :type "Actor Object Reference") (OtherComp :type "PrimitiveComponent Object Reference") (OtherBodyIndex :type Integer) (bFromSweep :type Boolean) (SweepResult :type "HitResult Structure (by ref)"))
  (cast `/Game/FirstPerson/Blueprints/BP_FirstPersonCharacter` OtherActor)
  (`GameplayStatics.ApplyDamage` self)
  (`GameplayStatics.PlaySound2D` "/Game/Enemies/Weapons/hit-sound.hit-sound" 1.0 1.0 0.0 null null))

(event `self.ReceiveAnyDamage`
  (params (Damage :type "Float (single-precision)") (DamageType :type "DamageType Object Reference") (InstigatedBy :type "Controller Object Reference") (DamageCauser :type "Actor Object Reference"))
  (bind _returnvalue (`self.GetTransform`))
  (bind _output_get (set `self.CurrentHealth` (- (`self.CurrentHealth`) (* Damage 5.0))))
  (`/Game/Enemies/WBP_EnemyHealth.UpdateHealth` (`self.WBP Enemy Health`) _output_get)
  (if (<= (`self.CurrentHealth`) 0)
    (if (<= (`KismetMathLibrary.RandomIntegerInRange` 0 10) 5)
      (`|SpawnActorFromClass` "/Game/Pickups/Ammo.Ammo_C" _returnvalue "Undefined" "MultiplyWithRoot" null null)
      (else
        (`|SpawnActorFromClass` "/Game/Pickups/HealthPickup.HealthPickup_C" _returnvalue "Undefined" "MultiplyWithRoot" null null)))
    (`self.K2_DestroyActor`)))

(event `Attack`
  (bind _notifyname (`|PlayMontage` (`self.Mesh`) "/Game/Enemies/Anims/ANIMATIONS/NEW_CAST_Montage.NEW_CAST_Montage")
    (:`OnNotifyBegin`
      (switch `name` _notifyname))))

(fn `Get Ideal Range`
  (returns (`Attack Radius` :type "Float (double-precision)"))
  (return 600.0))

(fn `SetMovementSpeed2`
  (params (Speed :type "/Game/Enemies/E_MovementSpeed Enum" :default "NewEnumerator0"))
  (returns (SpeedValue :type "Float (double-precision)"))
  (bind _output_get (set `CharacterMovementComponent.MaxWalkSpeed` (select `/Game/Enemies/E_MovementSpeed` Speed :`NewEnumerator1` 100.0 :`NewEnumerator2` 300.0 :`NewEnumerator3` 500.0 :!type "Float (single-precision)") (`self.CharacterMovement`)))
  (return _output_get))

(fn `UserConstructionScript`)